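; Monster character that switches from its normal mesh to a faster spider form and chases the player on sight.
; Pawn sensing and a trigger sphere drive AIMoveTo toward the player, while heard noises send it to their location (marked unfinished).
; CatchRange overlap plays an attack montage and calls OnCaught on the player, gated by a DoOnce with delayed reset.
; The logic to revert form and clear chasing is disconnected, so spider form persists.
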(event `self.PawnSensing.OnSeePawn`
  (params (Pawn :type "Pawn Object Reference"))
  ;[0.15 0.005984 0.06722 0.5] 시야감지 추격
  (bind _asbp_player_character (cast `/Game/Blueprints/Character/BP_PlayerCharacter` Pawn))
  (`self.SetMonsterForm` true)
  (set `self.IsChasing` true)
  (bind _asaicontroller (cast `AIController` (`self.GetController`)))
  (`Controller.StopMovement` _asaicontroller)
  (bind _output_get (set `self.LastSeenLocation` (`self.K2_GetActorLocation` _asbp_player_character)))
  (`|AIMoveTo` self (0.0 0.0 0.0) _asbp_player_character 150.0) ; 네비게이션 데이터로 경로를 계산하여 이동
)

(event `self.ReceiveBeginPlay`
  (`SkeletalMeshComponent.SetAnimInstanceClass` (`self.SpiderMesh`) "/Game/Blueprints/Monster/ABP_Monster_Spider.ABP_Monster_Spider_C")
  (`SceneComponent.SetHiddenInGame` (`self.SpiderMesh`) true false))

(event `self.Sphere.OnComponentBeginOverlap`
  (params (OverlappedComponent :type "PrimitiveComponent Object Reference") (OtherActor :type "Actor Object Reference") (OtherComp :type "PrimitiveComponent Object Reference") (OtherBodyIndex :type Integer) (bFromSweep :type Boolean) (SweepResult :type "HitResult Structure (by ref)"))
  ;[0.15 0.005984 0.06722 0.5] 시야감지 추격
  (bind _asbp_player_character (cast `/Game/Blueprints/Character/BP_PlayerCharacter` OtherActor))
  (`|AIMoveTo` self (0.0 0.0 0.0) _asbp_player_character 150.0) ; 네비게이션 데이터로 경로를 계산하여 이동
)

(event `self.CatchRange.OnComponentBeginOverlap`
  (params (OverlappedComponent :type "PrimitiveComponent Object Reference") (OtherActor :type "Actor Object Reference") (OtherComp :type "PrimitiveComponent Object Reference") (OtherBodyIndex :type Integer) (bFromSweep :type Boolean) (SweepResult :type "HitResult Structure (by ref)"))
  ;[0.15 0 0.0285 0.5] 플레이어 피격 + 애니메이션 재생  / 플레이어 이벤트 호출
  (`/Engine/EditorBlueprintResources/StandardMacros.DoOnce` false :!label _label
    (:`Completed`
      (bind _asbp_player_character (cast `/Game/Blueprints/Character/BP_PlayerCharacter` OtherActor))
      ;; 공격 모드일때만 재생
      (`AnimInstance.Montage_Play` (`SkeletalMeshComponent.GetAnimInstance` (`self.SpiderMesh`)) "/Game/Blueprints/Assets/Monster/little_nightmares_3__supervisor/SkeletalMeshes/AM_MonsterAttack.AM_MonsterAttack" 1.0 "MontageLength" 0.0 true)
      (`/Game/Blueprints/Character/BP_PlayerCharacter.OnCaught` _asbp_player_character)
      (`KismetSystemLibrary.Delay` 5.0)
      (goto _label :!via `Reset`))))

(event `self.PawnSensing.OnHearNoise`
  (params (Instigator :type "Pawn Object Reference") (Location :type "Vector Structure (by ref)") (Volume :type "Float (single-precision)"))
  ;[0.09244 0.15 0.04908 0.5] 소리감지 추격(미완성)
  (`|AIMoveTo` self Location null 1.0))

(fn `SetMonsterForm`
  (params (IsSpider :type Boolean))
  (if IsSpider
    ; spider 모드
    (`SceneComponent.SetHiddenInGame` (`self.Mesh`) true false)
    (`SceneComponent.SetHiddenInGame` (`self.SpiderMesh`) false false)
    (`SkeletalMeshComponent.SetAnimInstanceClass` (`self.SpiderMesh`) "/Game/Blueprints/Monster/ABP_Monster_Spider.ABP_Monster_Spider_C")
    (set `CharacterMovementComponent.MaxWalkSpeed` 900.0 (`self.CharacterMovement`))
    (else
      (`SceneComponent.SetHiddenInGame` (`self.SpiderMesh`) true false)
      (`SceneComponent.SetHiddenInGame` (`self.Mesh`) false false)
      (set `CharacterMovementComponent.MaxWalkSpeed` 500.0 (`self.CharacterMovement`)))))

(fn `UserConstructionScript`)