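; BP_PlayerCharacter is the player character Blueprint, handling movement, look and jump through Enhanced Input actions.
; IA_Move adds movement along right and forward vectors built from control rotation yaw alone, so camera pitch does not affect direction.
; IA_Look feeds controller yaw and pitch, while IA_Jump starts and stops the built-in character jump.
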(event `self.ReceiveBeginPlay`)

(event `EnhancedInput|/Game/Input/Actions/IA_Move`
  (params (ActionValue :type "Vector2D Structure") (ElapsedSeconds :type "Float (double-precision)") (TriggeredSeconds :type "Float (double-precision)") (InputAction :type "InputAction Object Reference" :default "/Game/Input/Actions/IA_Move.IA_Move"))
  (bind _returnvalue (`KismetMathLibrary.MakeRotator` 0.0 0.0 (.yaw (`self.GetControlRotation`))))
  ;[0 0.02281 0.15 0.5] 이동
  (:`Triggered`
    (`self.AddMovementInput` (`KismetMathLibrary.GetRightVector` _returnvalue) ActionValue_X)
    (`self.AddMovementInput` (`KismetMathLibrary.GetForwardVector` _returnvalue) ActionValue_Y)))

(event `EnhancedInput|/Game/Input/Actions/IA_Look`
  (params (ActionValue :type "Vector2D Structure") (ElapsedSeconds :type "Float (double-precision)") (TriggeredSeconds :type "Float (double-precision)") (InputAction :type "InputAction Object Reference" :default "/Game/Input/Actions/IA_Look.IA_Look"))
  ;[0 0.15 0.1175 0.5] 카메라 회전
  (:`Triggered`
    (`self.AddControllerYawInput` ActionValue_X) ; 좌우 돌리기
    (`self.AddControllerPitchInput` ActionValue_Y) ; 상하 돌리기
  ))

(event `EnhancedInput|/Game/Input/Actions/IA_Jump`
  (params (ActionValue :type Boolean) (ElapsedSeconds :type "Float (double-precision)") (TriggeredSeconds :type "Float (double-precision)") (InputAction :type "InputAction Object Reference" :default "/Game/Input/Actions/IA_Jump.IA_Jump"))
  ;[0.15 0.1174 0.005971 0.5] 점프
  (:`Started`
    (`self.Jump`))
  (:`Completed`
    (`self.StopJumping`)))

(fn `UserConstructionScript`)