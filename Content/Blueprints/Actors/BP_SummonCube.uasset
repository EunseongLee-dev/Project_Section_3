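; BP_SummonCube is a cube actor with an event that plays out its disappearance and then destroys it.
; DisappearAndDestroy turns off the box's physics and collision, then plays the cube mesh's animation once at a raised play rate.
; After a short delay, a timeline's alpha drives the actor's uniform scale, and the actor destroys itself when the timeline finishes.
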(event `DisappearAndDestroy`
  (bind _cubemesh (`self.CubeMesh`))
  (`PrimitiveComponent.SetSimulatePhysics` (`self.Box`) false)
  (`PrimitiveComponent.SetCollisionEnabled` (`self.Box`) "NoCollision")
  (`SkeletalMeshComponent.SetPlayRate` _cubemesh 10.0)
  (`SkeletalMeshComponent.PlayAnimation` _cubemesh "/Game/Blueprints/Assets/Cube/placeholder-cube_green/SkeletalMeshes/placeholder-cube_green_Anim.placeholder-cube_green_Anim" false)
  (`KismetSystemLibrary.Delay` 1.5)
  (bind (_direction _alpha) (`Timeline|FadeOutTimeline` :!via `PlayFromStart`)
    (:`Update`
      (`self.SetActorScale3D` (`KismetMathLibrary.Conv_DoubleToVector` _alpha)))
    (:`Finished`
      (`self.K2_DestroyActor`))))

(fn `UserConstructionScript`)