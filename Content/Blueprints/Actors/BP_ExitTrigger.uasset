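; BP_ExitTrigger is a level exit that only responds when the player character overlaps its Box while holding at least three souls.
; An exit flagged as final shows the victory widget, reveals the mouse cursor and switches to UI-only input.
; Any other exit adds a fade widget, waits briefly, then opens the hard-coded level Lvl_Room02.
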(event `self.Box.OnComponentBeginOverlap`
  (params (OverlappedComponent :type "PrimitiveComponent Object Reference") (OtherActor :type "Actor Object Reference") (OtherComp :type "PrimitiveComponent Object Reference") (OtherBodyIndex :type Integer) (bFromSweep :type Boolean) (SweepResult :type "HitResult Structure (by ref)"))
  (bind _returnvalue (`GameplayStatics.GetPlayerController` 0))
  (bind _asbp_player_character (cast `/Game/Blueprints/Character/BP_PlayerCharacter` OtherActor))
  (if (>= (`/Game/Blueprints/Character/BP_PlayerCharacter.SoulCount` _asbp_player_character) 3)
    (if (`self.blsFinalExit`)
      (bind _returnvalue_2 (`|CreateWidget` "/Game/Blueprints/UI/WBP_Victory.WBP_Victory_C"))
      (`UserWidget.AddToViewport` _returnvalue_2 0)
      (set `PlayerController.bShowMouseCursor` true _returnvalue)
      (`WidgetBlueprintLibrary.SetInputMode_UIOnlyEx` _returnvalue _returnvalue_2)
      (else
        (bind _returnvalue_3 (`|CreateWidget` "/Game/Blueprints/UI/WBP_Fade.WBP_Fade_C"))
        (`UserWidget.AddToViewport` _returnvalue_3 0)
        (`KismetSystemLibrary.Delay` 1.5)
        (`GameplayStatics.OpenLevel` "Lvl_Room02")))))

(fn `UserConstructionScript`)